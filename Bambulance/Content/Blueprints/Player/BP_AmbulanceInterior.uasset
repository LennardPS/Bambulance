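; BP_AmbulanceInterior is a player-side Blueprint for the ambulance interior that sets up mouse-driven interaction and the health UI.
; BeginPlay shows the mouse cursor and adds the WBP_Health widget to the viewport.
; Left mouse press sets IsGrabbed and runs a debug-drawn complex Visibility trace from the deprojected cursor; release clears the flag.
; The trace result is unused, so no grab behavior follows.
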(event `self.ReceiveBeginPlay`
  (set `PlayerController.bShowMouseCursor` true (`GameplayStatics.GetPlayerController` 0))
  (bind _returnvalue (`|CreateWidget` "/Game/Blueprints/UI/WBP_Health.WBP_Health_C"))
  (`UserWidget.AddToViewport` _returnvalue 0))

(event `Key|LeftMouseButton`
  (params (Key :type "Key Structure"))
  (bind (_worldlocation _worlddirection) (`PlayerController.DeprojectMousePositionToWorld` (`GameplayStatics.GetPlayerController` 0)))
  (:`Pressed`
    (set `self.IsGrabbed` true)
    (if (`self.IsGrabbed`)
      (`KismetSystemLibrary.LineTraceSingle` :`Start` _worldlocation :`End` (+ _worldlocation (* _worlddirection 10000.0)) :`TraceChannel` "TraceTypeQuery1" :`bTraceComplex` true :`DrawDebugType` "ForDuration")))
  (:`Released`
    (set `self.IsGrabbed` false)))

(fn `UserConstructionScript`)