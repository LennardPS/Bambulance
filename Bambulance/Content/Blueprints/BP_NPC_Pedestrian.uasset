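; BP_NPC_Pedestrian is a pedestrian NPC that roams at random and ragdolls when struck by a vehicle.
; From BeginPlay it uses AIMoveTo toward random reachable points, pausing and repeating after each successful move until hit.
; Capsule overlap with an NPC vehicle or ambulance driver enables physics on mesh and sphere, disables capsule collision, then destroys the pedestrian after a delay.
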(event `self.ReceiveBeginPlay`
  (`self.CE_StartMoving` true))

(event `CE_StartMoving`
  (params (`With Start Delay` :type Boolean))
  (if (not (`self.Was Hit`)) :!label _label
    (if `With Start Delay`
      ;[1 1 1] NPC Random Roaming
      (`KismetSystemLibrary.Delay` (`KismetMathLibrary.RandomFloatInRange` 0.0 1.0)))
    (set `self.Is Moving` true)
    (`|AIMoveTo` self (`NavigationSystemV1.K2_GetRandomReachablePointInRadius` (`self.K2_GetActorLocation` self) 10000.0 null null) null
      (:`OnSuccess`
        (set `self.Is Moving` false)
        ;[1 1 1] Resume Walking
        (`KismetSystemLibrary.Delay` (`self.TimeBeforeNextMove`))
        (goto _label)))))

(event `self.Capsule_Collision.OnComponentBeginOverlap`
  (params (OverlappedComponent :type "PrimitiveComponent Object Reference") (OtherActor :type "Actor Object Reference") (OtherComp :type "PrimitiveComponent Object Reference") (OtherBodyIndex :type Integer) (bFromSweep :type Boolean) (SweepResult :type "HitResult Structure (by ref)"))
  (bind _returnvalue (`GameplayStatics.GetObjectClass` OtherActor))
  ;[1 1 1] Ragdoll
  (if (or (== _returnvalue "/Game/Blueprints/BP_NPC_Vehicle.BP_NPC_Vehicle_C") (== _returnvalue "/Game/Blueprints/Player/BP_AmbulanceDriver.BP_AmbulanceDriver_C"))
    (if (not (`self.Was Hit`))
      (`PrimitiveComponent.SetSimulatePhysics` (`self.Mesh`) true)
      (`PrimitiveComponent.SetSimulatePhysics` (`self.Sphere`) true)
      (`PrimitiveComponent.SetCollisionEnabled` (`self.CapsuleComponent`) "NoCollision")
      (set `self.Was Hit` true)
      (`KismetSystemLibrary.Delay` 5.0)
      (`self.K2_DestroyActor`))))

(fn `UserConstructionScript`)