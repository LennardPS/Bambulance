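; BP_Physic_Pole is a breakable street pole, apparently a lamppost, that gives way when a vehicle hits it.
; A capsule overlap checks whether the other actor's class is exactly BP_NPC_Vehicle or BP_AmbulanceDriver.
; The first such hit turns on physics simulation for the Head and Pole components, and a WasHit flag blocks repeat triggers.
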(event `self.Capsule_Collision.OnComponentBeginOverlap`
  (params (OverlappedComponent :type "PrimitiveComponent Object Reference") (OtherActor :type "Actor Object Reference") (OtherComp :type "PrimitiveComponent Object Reference") (OtherBodyIndex :type Integer) (bFromSweep :type Boolean) (SweepResult :type "HitResult Structure (by ref)"))
  (bind _returnvalue (`GameplayStatics.GetObjectClass` OtherActor))
  (if (or (== _returnvalue "/Game/Blueprints/BP_NPC_Vehicle.BP_NPC_Vehicle_C") (== _returnvalue "/Game/Blueprints/Player/BP_AmbulanceDriver.BP_AmbulanceDriver_C"))
    (if (not (`self.Was Hit`))
      (`PrimitiveComponent.SetSimulatePhysics` (`self.Head`) true)
      (`PrimitiveComponent.SetSimulatePhysics` (`self.Pole`) true)
      (set `self.Was Hit` true))))

(fn `UserConstructionScript`)