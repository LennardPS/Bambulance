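; Game mode for the ambulance game that ties the BP_AmbulanceDriver pawn's Health to whether a patient is aboard.
; AddPatient spawns a character above the driver, sets HasPatient and starts a looping timer that drains Health, or refills it once the flag clears.
; Space clears the flag, Q spawns a character without setting it, and any damage to the game mode actor zeroes driver Health.
; Debug prints and unwired older damage logic remain.
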(event `self.ReceiveTick`
  (params (DeltaSeconds :type "Float (single-precision)"))
  ;[1 1 1] OLD
)

(event `self.ReceiveAnyDamage`
  (params (Damage :type "Float (single-precision)") (DamageType :type "DamageType Object Reference") (InstigatedBy :type "Controller Object Reference") (DamageCauser :type "Actor Object Reference"))
  (bind _asbp_ambulance_driver (cast `/Game/Blueprints/Player/BP_AmbulanceDriver` (`GameplayStatics.GetPlayerPawn` 0)))
  (set `/Game/Blueprints/Player/BP_AmbulanceDriver.Health` 0.0 _asbp_ambulance_driver))

(event `AddPatient`
  (bind _asbp_ambulance_driver (cast `/Game/Blueprints/Player/BP_AmbulanceDriver` (`GameplayStatics.GetPlayerPawn` 0)))
  (bind _returnvalue (`KismetMathLibrary.MakeVector` (.x (.location (`SceneComponent.K2_GetComponentToWorld` (`Actor.RootComponent` _asbp_ambulance_driver)))) (.y (.location (`SceneComponent.K2_GetComponentToWorld` (`Actor.RootComponent` _asbp_ambulance_driver)))) (+ (.z (.location (`SceneComponent.K2_GetComponentToWorld` (`Actor.RootComponent` _asbp_ambulance_driver)))) 100.0)))
  (`|SpawnActorFromClass` "/Game/ThirdPerson/Blueprints/BP_ThirdPersonCharacter.BP_ThirdPersonCharacter_C" (`KismetMathLibrary.MakeTransform` _returnvalue) "AdjustIfPossibleButAlwaysSpawn" "OverrideRootScale" null null)
  ;[1 1 1] Patient
  (`KismetSystemLibrary.PrintString` (`KismetStringLibrary.Conv_VectorToString` _returnvalue))
  (bind _output_get (set `self.HasPatient` true))
  (bind _asbp_ambulance_driver_2 (cast `/Game/Blueprints/Player/BP_AmbulanceDriver` (`GameplayStatics.GetPlayerPawn` 0)))
  (if (`self.HasPatient`)
    (`KismetSystemLibrary.K2_SetTimerDelegate` (delegate `HealthManagement`) 0.01 true)
    (`KismetSystemLibrary.PrintString` (`KismetStringLibrary.Conv_BoolToString` _output_get))))

(event `HealthManagement`
  ;[1 1 1] Patient
  (if (`self.HasPatient`)
    (set `/Game/Blueprints/Player/BP_AmbulanceDriver.Health` (- (`/Game/Blueprints/Player/BP_AmbulanceDriver.Health` (stale `AddPatient` _asbp_ambulance_driver_2)) 0.01) (stale `AddPatient` _asbp_ambulance_driver_2))
    (else
      (bind _asbp_ambulance_driver (cast `/Game/Blueprints/Player/BP_AmbulanceDriver` (`GameplayStatics.GetPlayerPawn` 0)))
      (set `/Game/Blueprints/Player/BP_AmbulanceDriver.Health` (`KismetMathLibrary.FClamp` (+ (`/Game/Blueprints/Player/BP_AmbulanceDriver.Health` _asbp_ambulance_driver) 100.0) 0.0 100.0) _asbp_ambulance_driver))))

(event `self.ReceiveBeginPlay`
  (`self.EnableInput` (`GameplayStatics.GetPlayerController` 0)))

(event `Key|SpaceBar`
  (params (Key :type "Key Structure"))
  (:`Pressed`
    (set `self.HasPatient` false)
    (`KismetSystemLibrary.PrintString` "False")))

(event `Key|Q`
  (params (Key :type "Key Structure"))
  (:`Pressed`
    (bind _asbp_ambulance_driver (cast `/Game/Blueprints/Player/BP_AmbulanceDriver` (`GameplayStatics.GetPlayerPawn` 0)))
    (bind _returnvalue (`KismetMathLibrary.MakeVector` (.x (.location (`SceneComponent.K2_GetComponentToWorld` (`Actor.RootComponent` _asbp_ambulance_driver)))) (.y (.location (`SceneComponent.K2_GetComponentToWorld` (`Actor.RootComponent` _asbp_ambulance_driver)))) (+ (.z (.location (`SceneComponent.K2_GetComponentToWorld` (`Actor.RootComponent` _asbp_ambulance_driver)))) 100.0)))
    (`|SpawnActorFromClass` "/Game/ThirdPerson/Blueprints/BP_ThirdPersonCharacter.BP_ThirdPersonCharacter_C" (`KismetMathLibrary.MakeTransform` _returnvalue) "AdjustIfPossibleButAlwaysSpawn" "OverrideRootScale" null null)
    (`KismetSystemLibrary.PrintString` (`KismetStringLibrary.Conv_VectorToString` _returnvalue))))

(fn `UserConstructionScript`)