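; Player-driven, physics-based ambulance that creates a minimap widget on BeginPlay.
; Held WASD or Left/Right keys run Timelines that push and torque the wheel bodies, mostly scaled by speed curves, while steering also angles the front wheel meshes.
; Tick line-traces both axles for grounding, derives KPH and reversing state to steer those forces, and applies counter-drift grip when the rear is grounded.
; Debug traces, speed and traction-curve readouts are active.
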(event `self.ReceiveBeginPlay`
  (bind _returnvalue (`|CreateWidget` "/Game/Blueprints/UI/WBP_Minimap.WBP_Minimap_C"))
  (`UserWidget.AddToViewport` _returnvalue 0))

(event `Key|Left` :consume false
  (params (Key :type "Key Structure"))
  (bind _fr_mesh (`self.FR_Mesh`))
  (:`Pressed`
    (`SceneComponent.K2_SetRelativeRotation` _fr_mesh (`KismetMathLibrary.MakeRotator` -90.0 0.0 -9.0) false false :!label _label)
    (`SceneComponent.K2_SetRelativeRotation` (`self.FL_Mesh`) (`KismetMathLibrary.MakeRotator` -90.0 0.0 -9.0) false false))
  (:`Released`
    (`SceneComponent.K2_SetRelativeRotation` _fr_mesh (`KismetMathLibrary.MakeRotator` -90.0) false false :!label _label_2)
    (`SceneComponent.K2_SetRelativeRotation` (`self.FL_Mesh`) (`KismetMathLibrary.MakeRotator` -90.0) false false)))

(event `Key|A` :consume false
  (params (Key :type "Key Structure"))
  (:`Pressed`
    (goto _label))
  (:`Released`
    (goto _label_2)))

(event `Key|S` :consume false
  (params (Key :type "Key Structure"))
  ;[1 1 1] Brake Reverse
  (:`Pressed`
    (`/Engine/EditorBlueprintResources/StandardMacros.DoOnce` false :!label _label_3
      (:`Completed`
        (`Timeline|Timeline_3` :!via `PlayFromStart` :!label _label_4
          (:`Update`
            (if (`self.IsRearGrounded`)
              (if (`self.IsReversing`)
                (`PrimitiveComponent.AddForce` (`self.BR_Wheel`) (* (* (`SceneComponent.GetForwardVector` (`self.Body`)) (* (`self.ReversingForce`) (`CurveFloat.GetFloatValue` (`self.CurveMaxReverse`) (`self.KPH`)))) (-1.0 -1.0 -1.0)) "None" false)
                (`PrimitiveComponent.AddForce` (`self.BL_Wheel`) (* (* (`SceneComponent.GetForwardVector` (`self.Body`)) (* (`self.ReversingForce`) (`CurveFloat.GetFloatValue` (`self.CurveMaxReverse`) (`self.KPH`)))) (-1.0 -1.0 -1.0)) "None" false)
                (else
                  (`PrimitiveComponent.AddForce` (`self.FL_Wheel`) (* (* (`SceneComponent.GetForwardVector` (`self.Body`)) (`self.DeccelerationForce`)) (-1.0 -1.0 -1.0)) "None" false)
                  (`PrimitiveComponent.AddForce` (`self.FR_Wheel`) (* (* (`SceneComponent.GetForwardVector` (`self.Body`)) (`self.DeccelerationForce`)) (-1.0 -1.0 -1.0)) "None" false)))))))))
  (:`Released`
    (`|ExecutionSequence`
      (:`then_0`
        (goto _label_3 :!via `Reset`))
      (:`then_1`
        (goto _label_4 :!via `Stop`)))))

(event `Key|Left` :consume false
  (params (Key :type "Key Structure"))
  ;[1 1 1] Manual Steering
  (:`Pressed`
    (`Timeline|Timeline_1` :!via `PlayFromStart` :!label _label_5
      (:`Update`
        (if (`self.IsFrontGrounded`)
          (if (`self.IsReversing`)
            (`PrimitiveComponent.AddTorqueInDegrees` (`self.FR_Wheel`) (`KismetMathLibrary.MakeVector` 0.0 0.0 (* (`self.TurnForce`) (`CurveFloat.GetFloatValue` (`self.CurveTurn`) (`self.KPH`)))) "None" false)
            (`PrimitiveComponent.AddTorqueInDegrees` (`self.FL_Wheel`) (`KismetMathLibrary.MakeVector` 0.0 0.0 (* (`self.TurnForce`) (`CurveFloat.GetFloatValue` (`self.CurveTurn`) (`self.KPH`)))) "None" false)
            (else
              (`PrimitiveComponent.AddTorqueInDegrees` (`self.FL_Wheel`) (`KismetMathLibrary.MakeVector` 0.0 0.0 (* (* (`self.TurnForce`) (`CurveFloat.GetFloatValue` (`self.CurveTurn`) (`self.KPH`))) -1.0)) "None" false)
              (`PrimitiveComponent.AddTorqueInDegrees` (`self.FR_Wheel`) (`KismetMathLibrary.MakeVector` 0.0 0.0 (* (* (`self.TurnForce`) (`CurveFloat.GetFloatValue` (`self.CurveTurn`) (`self.KPH`))) -1.0)) "None" false)))))))
  (:`Released`
    (goto _label_5 :!via `Stop`)))

(event `Key|A` :consume false
  (params (Key :type "Key Structure"))
  ;[1 1 1] Manual Steering
  (:`Pressed`
    (goto _label_5 :!via `PlayFromStart`))
  (:`Released`
    (goto _label_5 :!via `Stop`)))

(event `Key|Right` :consume false
  (params (Key :type "Key Structure"))
  ;[1 1 1] Manual Steering
  (:`Pressed`
    (`Timeline|Timeline_2` :!via `PlayFromStart` :!label _label_6
      (:`Update`
        (if (`self.IsFrontGrounded`)
          (if (`self.IsReversing`)
            (`PrimitiveComponent.AddTorqueInDegrees` (`self.FL_Wheel`) (`KismetMathLibrary.MakeVector` 0.0 0.0 (* (* (`self.TurnForce`) (`CurveFloat.GetFloatValue` (`self.CurveTurn`) (`self.KPH`))) -1.0)) "None" false)
            (`PrimitiveComponent.AddTorqueInDegrees` (`self.FR_Wheel`) (`KismetMathLibrary.MakeVector` 0.0 0.0 (* (* (`self.TurnForce`) (`CurveFloat.GetFloatValue` (`self.CurveTurn`) (`self.KPH`))) -1.0)) "None" false)
            (else
              (`PrimitiveComponent.AddTorqueInDegrees` (`self.FL_Wheel`) (`KismetMathLibrary.MakeVector` 0.0 0.0 (* (`self.TurnForce`) (`CurveFloat.GetFloatValue` (`self.CurveTurn`) (`self.KPH`)))) "None" false)
              (`PrimitiveComponent.AddTorqueInDegrees` (`self.FR_Wheel`) (`KismetMathLibrary.MakeVector` 0.0 0.0 (* (`self.TurnForce`) (`CurveFloat.GetFloatValue` (`self.CurveTurn`) (`self.KPH`)))) "None" false)))))))
  (:`Released`
    (goto _label_6 :!via `Stop`)))

(event `Key|D` :consume false
  (params (Key :type "Key Structure"))
  ;[1 1 1] Manual Steering
  (:`Pressed`
    (goto _label_6 :!via `PlayFromStart`))
  (:`Released`
    (goto _label_6 :!via `Stop`)))

(event `Key|Right` :consume false
  (params (Key :type "Key Structure"))
  (bind _fr_mesh (`self.FR_Mesh`))
  (:`Pressed`
    (`SceneComponent.K2_SetRelativeRotation` _fr_mesh (struct :`Yaw` 9.0 :`Roll` -90.0) false false :!label _label_7)
    (`SceneComponent.K2_SetRelativeRotation` (`self.FL_Mesh`) (struct :`Yaw` 9.0 :`Roll` -90.0) false false))
  (:`Released`
    (`SceneComponent.K2_SetRelativeRotation` _fr_mesh (struct :`Roll` -90.0) false false :!label _label_8)
    (`SceneComponent.K2_SetRelativeRotation` (`self.FL_Mesh`) (struct :`Roll` -90.0) false false)))

(event `Key|D` :consume false
  (params (Key :type "Key Structure"))
  (:`Pressed`
    (goto _label_7))
  (:`Released`
    (goto _label_8)))

(event `Key|W` :consume false
  (params (Key :type "Key Structure"))
  ;[1 1 1] Accelerate
  (:`Pressed`
    (`/Engine/EditorBlueprintResources/StandardMacros.DoOnce` false :!label _label_9
      (:`Completed`
        (`Timeline|Timeline_0` :!via `PlayFromStart` :!label _label_10
          (:`Update`
            (if (`self.IsRearGrounded`)
              (if (`self.IsReversing`)
                (`PrimitiveComponent.AddForce` (`self.BR_Wheel`) (* (`SceneComponent.GetForwardVector` (`self.Body`)) (* (`self.ReversingForce`) (`CurveFloat.GetFloatValue` (`self.CurveMaxSpeed`) (`self.KPH`)))) "None" false)
                (`PrimitiveComponent.AddForce` (`self.BL_Wheel`) (* (`SceneComponent.GetForwardVector` (`self.Body`)) (* (`self.ReversingForce`) (`CurveFloat.GetFloatValue` (`self.CurveMaxSpeed`) (`self.KPH`)))) "None" false)
                (else
                  (`PrimitiveComponent.AddForce` (`self.BR_Wheel`) (* (`SceneComponent.GetForwardVector` (`self.Body`)) (* (`self.DeccelerationForce`) (`CurveFloat.GetFloatValue` (`self.CurveMaxSpeed`) (`self.KPH`)))) "None" false)
                  (`PrimitiveComponent.AddForce` (`self.BL_Wheel`) (* (`SceneComponent.GetForwardVector` (`self.Body`)) (* (`self.DeccelerationForce`) (`CurveFloat.GetFloatValue` (`self.CurveMaxSpeed`) (`self.KPH`)))) "None" false)))))))))
  (:`Released`
    (`|ExecutionSequence`
      (:`then_0`
        (goto _label_9 :!via `Reset`))
      (:`then_1`
        (goto _label_10 :!via `Stop`)))))

(event `self.ReceiveTick`
  (params (DeltaSeconds :type "Float (single-precision)"))
  (`|ExecutionSequence`
    (:`then_0`
      (set `self.Delta Seconds` DeltaSeconds)
      (`self.F_GroundCheck`)
      (`self.F_CarVelocity`)
      (`self.F_Traction`))
    (:`then_1`
      (`KismetSystemLibrary.PrintString` (`KismetStringLibrary.Concat_StrStr` (`KismetStringLibrary.Conv_IntToString` (`KismetMathLibrary.Round` (`self.KPH`))) " KPH") true false (struct :`R` 0.204882 :`G` 1.0 :`A` 1.0) (`self.Delta Seconds`)))))

(fn `F_CarVelocity`
  (bind _returnvalue (`PrimitiveComponent.GetPhysicsLinearVelocity` (`self.Body`) "None"))
  (bind _output_get (set `self.LinearVelocity` _returnvalue))
  (set `self.IsReversing` (> 0.8 (`KismetMathLibrary.Dot_VectorVector` (`SceneComponent.GetForwardVector` (`self.Body`)) (`KismetMathLibrary.Normal` _output_get 0.09))))
  (set `self.KPH` (* (`KismetMathLibrary.VSize` _returnvalue) 0.036)))

(fn `F_GroundCheck`
  (bind _rearaxel (`self.RearAxel`))
  (bind _frontaxel (`self.FrontAxel`))
  (bind _returnvalue (* (`self.CarHeight`) -1.0))
  (bind _returnvalue_2 (* (`self.CarHeight`) -1.0))
  (bind (_outhit _returnvalue_3) (`KismetSystemLibrary.LineTraceSingleForObjects` :`Start` (`SceneComponent.K2_GetComponentLocation` _rearaxel) :`End` (+ (`SceneComponent.K2_GetComponentLocation` _rearaxel) (* (`SceneComponent.GetUpVector` (`self.Body`)) (`KismetMathLibrary.MakeVector` _returnvalue _returnvalue _returnvalue))) :`ObjectTypes` (`self.Ground Check Type`) :`DrawDebugType` "ForOneFrame"))
  (set `self.IsRearGrounded` _returnvalue_3)
  (bind (_outhit_2 _returnvalue_4) (`KismetSystemLibrary.LineTraceSingleForObjects` :`Start` (`SceneComponent.K2_GetComponentLocation` _frontaxel) :`End` (+ (`SceneComponent.K2_GetComponentLocation` _frontaxel) (* (`SceneComponent.GetUpVector` (`self.Body`)) (`KismetMathLibrary.MakeVector` _returnvalue_2 _returnvalue_2 _returnvalue_2))) :`ObjectTypes` (`self.Ground Check Type`) :`DrawDebugType` "ForOneFrame"))
  (set `self.IsFrontGrounded` _returnvalue_4))

(fn `F_Traction`
  (bind _grip (`self.Grip`))
  (bind _driftoffset (`self.DriftOffset`))
  (bind _body (`self.Body`))
  (set `self.DriftOffset` (`KismetMathLibrary.Dot_VectorVector` (`KismetMathLibrary.Normal` (`self.LinearVelocity`)) (`SceneComponent.GetRightVector` (`self.Body`))))
  (if (`self.IsRearGrounded`)
    (`PrimitiveComponent.AddForce` _body (* (* (`SceneComponent.GetRightVector` _body) (* _driftoffset -1.0)) (`KismetMathLibrary.MakeVector` _grip _grip _grip)) "None" false)
    (`KismetSystemLibrary.PrintString` (`KismetStringLibrary.Conv_DoubleToString` (`CurveFloat.GetFloatValue` (`self.CuveTraction`) _driftoffset)) true true (struct :`G` 0.66 :`B` 1.0 :`A` 1.0) (`self.Delta Seconds`))))

(fn `UserConstructionScript`)