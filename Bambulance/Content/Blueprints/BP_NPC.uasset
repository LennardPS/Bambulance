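; NPC car actor that drives along a referenced road spline in either direction.
; On BeginPlay it picks a random body material, caches the spline length and flips the mesh 180 degrees if the direction is inverted.
; A timeline, with play rate set by TimeToComplete and start time by StartingOffset, interpolates spline distance to update the actor's world location and rotation.
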(event `self.ReceiveBeginPlay`
  ;[1 1 1] Set Material
  (`PrimitiveComponent.SetMaterial` (`self.BodyMesh`) 0 (`|GetArrayItem` (`self.Materials`) (`KismetMathLibrary.RandomIntegerInRange` 0 7)))
  ;[1 1 1] Set Variables
  (set `self.Spline Length` (`SplineComponent.GetSplineLength` (`/Game/Blueprints/BP_RoadSpline.Spline` (`self.Road Spline`))))
  (if (`self.Inverse Direction`)
    (`SceneComponent.K2_SetRelativeRotation` (`self.BodyMesh`) (struct :`Yaw` 180.0) false false))
  ;[1 1 1] Move Car
  (`self.Move Car`))

(event `Move Car`
  (bind _spline_length (`self.Spline Length`))
  (bind _inverse_direction (`self.Inverse Direction`))
  (bind _spline (`/Game/Blueprints/BP_RoadSpline.Spline` (`self.Road Spline`)))
  ;[1 1 1] Move Car
  (`TimelineComponent.SetPlayRate` (`self.Timeline Move Object`) (/ 1.0 (`self.Time To Complete`)))
  (`TimelineComponent.SetNewTime` (`self.Timeline Move Object`) (`self.Starting Offset`))
  (bind (_direction _move_track) (`Timeline|Timeline Move Object`)
    (:`Update`
      (bind _returnvalue (`KismetMathLibrary.Lerp` (`KismetMathLibrary.SelectFloat` _spline_length 0.0 _inverse_direction) (`KismetMathLibrary.SelectFloat` 0.0 _spline_length _inverse_direction) _move_track))
      (`self.K2_SetActorTransform` (`KismetMathLibrary.MakeTransform` (`SplineComponent.GetLocationAtDistanceAlongSpline` _spline _returnvalue "World") (`SplineComponent.GetRotationAtDistanceAlongSpline` _spline _returnvalue "World"))))))

(fn `UserConstructionScript`)