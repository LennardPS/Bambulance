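; BP_NPC_Vehicle is an NPC traffic car with a random body material that, unless static, follows a road spline in either direction.
; A timeline drives its position and rotation along the spline.
; A front trigger tracks vehicles or the ambulance ahead, eases the car to a stop, and polls until the path clears.
; An ambulance hitting its hitbox stops it, turns its parts into physics bodies, and destroys it after a delay.
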(event `self.ReceiveBeginPlay`
  ;[1 1 1] Set Material
  (`PrimitiveComponent.SetMaterial` (`self.BodyMesh`) 0 (`|GetArrayItem` (`self.Materials`) (`KismetMathLibrary.RandomIntegerInRange` 0 7)))
  ;[1 1 1] Set Parts
  (set `self.Car Parts` (`|MakeArray` (`self.FL_Mesh`) (`self.FR_Mesh`) (`self.BL_Mesh`) (`self.BR_Mesh`) (`self.BodyMesh`)))
  (if (not (`self.Is Static`))
    ;[1 1 1] Set Variables
    (set `self.Spline Length` (`SplineComponent.GetSplineLength` (`/Game/Blueprints/BP_RoadSpline.Spline` (`self.Road Spline`))))
    (set `self.Play Rate` (/ 1.0 (`self.Time To Complete`)))
    (if (`self.Inverse Direction`)
      (`SceneComponent.K2_SetRelativeRotation` (`self.BodyMesh`) (struct :`Yaw` 180.0) false false))
    ;[1 1 1] Move Car
    (`self.CE_CarStartMoving`)))

(event `CE_CarStartMoving`
  (bind _spline_length (`self.Spline Length`))
  (bind _inverse_direction (`self.Inverse Direction`))
  (bind _spline (`/Game/Blueprints/BP_RoadSpline.Spline` (`self.Road Spline`)))
  ;[1 1 1] Move Car
  (`TimelineComponent.SetNewTime` (`self.Timeline Move Object`) (`self.Starting Offset`))
  (`TimelineComponent.SetPlayRate` (`self.Timeline Move Object`) (`self.Play Rate`) :!label _label)
  (set `self.Is Stopped` false)
  (bind (_direction _move_track) (`Timeline|Timeline Move Object` :!label _label_2)
    (:`Update`
      (bind _returnvalue (`KismetMathLibrary.Lerp` (`KismetMathLibrary.SelectFloat` _spline_length 0.0 _inverse_direction) (`KismetMathLibrary.SelectFloat` 0.0 _spline_length _inverse_direction) _move_track))
      (`self.K2_SetActorTransform` (`KismetMathLibrary.MakeTransform` (`SplineComponent.GetLocationAtDistanceAlongSpline` _spline _returnvalue "World") (`SplineComponent.GetRotationAtDistanceAlongSpline` _spline _returnvalue "World"))))))

(event `CE_CarResumeMoving`
  ;[1 1 1] Move Car
  (goto _label))

(event `CE_CarStopMoving`
  ;[1 1 1] Move Car
  (`TimelineComponent.SetPlayRate` (`self.Timeline Move Object`) 0.0)
  (set `self.Is Stopped` true)
  (goto _label_2 :!via `Stop`))

(event `self.Collision_Hitbox.OnComponentBeginOverlap`
  (params (OverlappedComponent :type "PrimitiveComponent Object Reference") (OtherActor :type "Actor Object Reference") (OtherComp :type "PrimitiveComponent Object Reference") (OtherBodyIndex :type Integer) (bFromSweep :type Boolean) (SweepResult :type "HitResult Structure (by ref)"))
  ;[1 1 1] Hit Collision
  (if (== (`GameplayStatics.GetObjectClass` OtherActor) "/Game/Blueprints/Player/BP_AmbulanceDriver.BP_AmbulanceDriver_C")
    (if (not (`self.Is Crashed`))
      (set `self.Is Crashed` true)
      (`self.CE_CarStopMoving`)
      (`PrimitiveComponent.SetCollisionEnabled` (`self.Collision_Front`) "NoCollision")
      ;[1 1 1] Set Physic
      (for _array_element (`self.Car Parts`)
        (`PrimitiveComponent.SetSimulatePhysics` _array_element true)
        ;[1 1 1] Clean Body
        (`KismetSystemLibrary.Delay` (`self.Time Before Cleanup`))
        (`self.CE_CleanBody`)))))

(event `self.Collision_Front.OnComponentBeginOverlap`
  (params (OverlappedComponent :type "PrimitiveComponent Object Reference") (OtherActor :type "Actor Object Reference") (OtherComp :type "PrimitiveComponent Object Reference") (OtherBodyIndex :type Integer) (bFromSweep :type Boolean) (SweepResult :type "HitResult Structure (by ref)"))
  (bind _returnvalue (`GameplayStatics.GetObjectClass` OtherActor))
  ;[1 1 1] Front Detection Stop & Resume
  (if (or (== _returnvalue "BP_NPC_Vehicle_C") (== _returnvalue "/Game/Blueprints/Player/BP_AmbulanceDriver.BP_AmbulanceDriver_C"))
    (`KismetArrayLibrary.Array_AddUnique` (`self.Cars In Front`) OtherActor)
    (if (not (`self.Is Stopped`))
      (bind (_direction _newtrack_0) (`Timeline|Timeline Slow Down`)
        (:`Update`
          (`TimelineComponent.SetPlayRate` (`self.Timeline Move Object`) (`KismetMathLibrary.Lerp` (`self.Play Rate`) 0.0 _newtrack_0)))
        (:`Finished`
          (`self.CE_CarStopMoving`)
          (`self.CE_CheckTraffic` 5.0))))))

(event `self.Collision_Front.OnComponentEndOverlap`
  (params (OverlappedComponent :type "PrimitiveComponent Object Reference") (OtherActor :type "Actor Object Reference") (OtherComp :type "PrimitiveComponent Object Reference") (OtherBodyIndex :type Integer))
  (bind _cars_in_front (`self.Cars In Front`))
  ;[1 1 1] Front Detection Stop & Resume
  (`KismetArrayLibrary.Array_RemoveItem` _cars_in_front OtherActor)
  (if (`KismetArrayLibrary.Array_IsEmpty` _cars_in_front)
    (`KismetSystemLibrary.Delay` 1.0)
    (`self.CE_CarResumeMoving`)))

(event `CE_CheckTraffic`
  (params (Delay :type "Float (double-precision)" :default 2.0))
  ;[1 1 1] Check Traffic
  (`KismetSystemLibrary.Delay` Delay :!label _label_3)
  (if (`KismetArrayLibrary.Array_IsEmpty` (`self.Cars In Front`))
    (`self.CE_CarResumeMoving`)
    (else
      (goto _label_3))))

(event `CE_CleanBody`
  ;[1 1 1] Destroy Actor
  (`self.K2_DestroyActor`))

(fn `UserConstructionScript`)